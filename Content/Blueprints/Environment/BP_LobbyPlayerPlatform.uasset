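; Lobby platform actor that represents one player slot, spawning and removing a BP_ThirdPersonCharacter with its lobby info widget for a given PlayerController.
; An empty slot shows a friend list button widget, which setup on BeginPlay links back to the platform on the server only.
; ShowFriendList moves the BP_FriendList actor found in the level to this platform, and spawning a character hides it if it is there.
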(event `SpawnCharacter`
  (params (PlayerController :type "PlayerController Object Reference"))
  (bind _currentcharacter (`self.CurrentCharacter`))
  (set `self.PlayerController` PlayerController)
  (`/Engine/EditorBlueprintResources/StandardMacros.IsValid` _currentcharacter
    (:`Is Valid`
      (`self.K2_DestroyActor` _currentcharacter))
    (:`Is Not Valid`
      _))
  (bind _returnvalue (`|SpawnActorFromClass` "/Game/ThirdPerson/Blueprints/BP_ThirdPersonCharacter.BP_ThirdPersonCharacter_C" (`SceneComponent.K2_GetComponentToWorld` (`self.PlayerSpawnTransform`)) "Undefined" "MultiplyWithRoot" null null))
  (set `self.CurrentCharacter` _returnvalue)
  (`/Game/ThirdPerson/Blueprints/BP_ThirdPersonCharacter.ShowLobbyInfoWidget` _returnvalue)
  (`SceneComponent.SetVisibility` (`self.ShowFriendListButton`) false false)
  (if (== (`self.K2_GetActorLocation` (`self.FriendListRef`)) (`SceneComponent.K2_GetComponentLocation` (`self.FriendListLocation`)) :`ErrorTolerance` 1.0)
    (`/Game/Blueprints/Environment/BP_FriendList.Show` (`self.FriendListRef`) false null)))

(event `RemoveCharacter`
  (bind _currentcharacter (`self.CurrentCharacter`))
  (set `self.PlayerController` null)
  (`/Engine/EditorBlueprintResources/StandardMacros.IsValid` _currentcharacter
    (:`Is Valid`
      (`self.K2_DestroyActor` _currentcharacter))
    (:`Is Not Valid`
      _))
  (`SceneComponent.SetVisibility` (`self.ShowFriendListButton`) true false))

(event `self.ReceiveBeginPlay`
  (`self.SetupServer`))

(fn `SetupServer`
  (if (`KismetSystemLibrary.IsServer`)
    (bind _returnvalue (`GameplayStatics.GetActorOfClass` "/Game/Blueprints/Environment/BP_FriendList.BP_FriendList_C"))
    (set `self.FriendListRef` _returnvalue)
    (bind _aswbp_show_friend_list_button (cast `/Game/Blueprints/Widgets/WBP_ShowFriendListButton` (`WidgetComponent.GetWidget` (`self.ShowFriendListButton`))))
    (set `/Game/Blueprints/Widgets/WBP_ShowFriendListButton.LobbyPlayerPlatformRef` self _aswbp_show_friend_list_button)
    (`SceneComponent.SetVisibility` (`self.ShowFriendListButton`) true false)))

(fn `ShowFriendList`
  (params (bShow :type Boolean))
  (bind _returnvalue (`WidgetComponent.GetWidget` (`self.ShowFriendListButton`)))
  (if bShow
    (`Widget.SetVisibility` _returnvalue "Collapsed")
    (`self.K2_SetActorLocation` (`self.FriendListRef`) (`SceneComponent.K2_GetComponentLocation` (`self.FriendListLocation`)) false false)
    (`/Game/Blueprints/Environment/BP_FriendList.Show` (`self.FriendListRef`) true self)
    (else
      (`Widget.SetVisibility` _returnvalue "Visible"))))

(fn `UserConstructionScript`)