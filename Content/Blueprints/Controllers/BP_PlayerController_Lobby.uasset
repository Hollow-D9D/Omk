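; Lobby player controller that shows the lobby UI and reports the player's info and ready state to BP_GameMode_Lobby.
; On BeginPlay, the local controller creates the lobby widget, enables cursor and game-and-UI input, then registers through SetPlayerNameOnServer.
; Pressing R toggles Ready and updates the game mode, while a retry event repeats that update after a short delay.
; OnStartMatch shows the loading screen and disables input.
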(event `RetryUpdateLobbyInfo`
  (`KismetSystemLibrary.Delay` 0.1)
  (bind _asbp_game_mode_lobby (cast `/Game/Framework/BP_GameMode_Lobby` (`GameplayStatics.GetGameMode`)))
  (`/Game/Framework/BP_GameMode_Lobby.UpdatePlayerLobbyInfo` _asbp_game_mode_lobby self))

(event `self.ReceiveBeginPlay`
  (`self.Setup`))

(event `SetPlayerNameOnServer`
  (bind _asbp_game_mode_lobby (cast `/Game/Framework/BP_GameMode_Lobby` (`GameplayStatics.GetGameMode`)))
  (`/Game/Framework/BP_GameMode_Lobby.UpdatePlayerLobbyInfo` _asbp_game_mode_lobby self))

(event `ToggleReadyStatusOnServer`
  (set `self.bReady` (not (`self.bReady`)))
  (bind _asbp_game_mode_lobby (cast `/Game/Framework/BP_GameMode_Lobby` (`GameplayStatics.GetGameMode`))
    (:`then`
      (`/Game/Framework/BP_GameMode_Lobby.UpdatePlayerLobbyInfo` _asbp_game_mode_lobby self))
    (:`CastFailed`
      (`KismetSystemLibrary.PrintString` "Failed to update ready"))))

(event `Key|R`
  (params (Key :type "Key Structure"))
  (:`Pressed`
    (`self.ToggleReadyStatusOnServer`)))

(event `OnStartMatch`
  (`/Game/Blueprints/Widgets/WBP_LobbyUI.ShowLoadingScreen` (`self.LobbyUI_Ref`))
  (`self.DisableInput` self))

(fn `Setup`
  (if (`self.IsLocalPlayerController`)
    (set `self.bShowMouseCursor` true)
    (`WidgetBlueprintLibrary.SetInputMode_GameAndUIEx` self null "DoNotLock" false)
    (bind _returnvalue (`|CreateWidget` "/Game/Blueprints/Widgets/WBP_LobbyUI.WBP_LobbyUI_C"))
    (bind _output_get (set `self.LobbyUI_Ref` _returnvalue))
    (`UserWidget.AddToViewport` _output_get 0)
    (`self.SetPlayerNameOnServer`)))

(fn `UserConstructionScript`)