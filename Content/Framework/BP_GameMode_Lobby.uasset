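; Lobby game mode that shows joined players as characters on platforms and handles ready state, kicking and match start.
; At BeginPlay it collects platforms ordered by index tag; login waits for that setup, then login and logout both sync players to platforms.
; Lobby info updates reach each player's character, with retry if unplaced, and feed a readiness check into the first controller's UI.
; StartMatch server-travels to the gameplay map and notifies every controller.
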(event `self.ReceiveBeginPlay`
  (`self.SetUpPlatforms`))

(event `self.K2_PostLogin`
  (params (NewPlayer :type "PlayerController Object Reference"))
  (`KismetArrayLibrary.Array_AddUnique` (`self.PlayerControllers`) NewPlayer)
  (`self.IsPlatformSetupDone` :!label _label
    (:`true`
      (`self.UpdatePlayersOnPlatforms`))))

(event `self.K2_OnLogout`
  (params (ExitingController :type "Controller Object Reference"))
  (bind _asplayer_controller (cast `PlayerController` ExitingController))
  (`KismetArrayLibrary.Array_RemoveItem` (`self.PlayerControllers`) _asplayer_controller)
  (goto _label))

(fn `CanStartGame`
  (locals (AllPlayersReady :type Boolean :default true))
  (for _array_element (`self.PlayerControllers`)
    (bind _asbp_player_controller_lobby (cast `/Game/Blueprints/Controllers/BP_PlayerController_Lobby` _array_element))
    (if (not (`/Game/Blueprints/Controllers/BP_PlayerController_Lobby.bReady` _asbp_player_controller_lobby))
      (set `local.AllPlayersReady` false)))
  (set `/Game/Blueprints/Widgets/WBP_LobbyUI.bEnoughPlayersReady` (`local.AllPlayersReady`) (`/Game/Blueprints/Controllers/BP_PlayerController_Lobby.LobbyUI_Ref` (cast `/Game/Blueprints/Controllers/BP_PlayerController_Lobby` (`GameplayStatics.GetPlayerController` 0) :!pure true))))

(fn `KickPlayer`
  (params (PlayerToKick :type "PlayerController Object Reference"))
  (`AdvancedSessionsLibrary.KickPlayer` PlayerToKick "Tenc em uzum"))

(fn `SetUpPlatforms`
  (bind _outactors (`GameplayStatics.GetAllActorsOfClass` "/Game/Blueprints/Environment/BP_LobbyPlayerPlatform.BP_LobbyPlayerPlatform_C"))
  (for _index (range (+ (`KismetArrayLibrary.Array_LastIndex` _outactors) 1))
    (bind _outactors_2 (`GameplayStatics.GetAllActorsOfClassWithTag` "/Game/Blueprints/Environment/BP_LobbyPlayerPlatform.BP_LobbyPlayerPlatform_C" (`KismetStringLibrary.Conv_StringToName` (`KismetStringLibrary.Conv_IntToString` _index))))
    (`KismetArrayLibrary.Array_AddUnique` (`self.PlayerPlatforms`) (`|GetArrayItem` _outactors_2)))
  (set `self.bPlatformSetupDone` true))

(fn `StartMatch`
  (`AdvancedSessionsLibrary.ServerTravel` (`self.GameplayMapName`))
  (for _array_element (`self.PlayerControllers`)
    (bind _asbp_player_controller_lobby (cast `/Game/Blueprints/Controllers/BP_PlayerController_Lobby` _array_element))
    (`/Game/Blueprints/Controllers/BP_PlayerController_Lobby.OnStartMatch` _asbp_player_controller_lobby)))

(fn `UpdatePlayerLobbyInfo`
  (params (RequestingPlayerController :type "PlayerController Object Reference"))
  (bind _requestingplayercontroller (`local.RequestingPlayerController`))
  (for _array_element (`self.PlayerPlatforms`)
    (if (== (`/Game/Blueprints/Environment/BP_LobbyPlayerPlatform.PlayerController` _array_element) RequestingPlayerController)
      (bind _asbp_third_person_character (cast `/Game/ThirdPerson/Blueprints/BP_ThirdPersonCharacter` (`/Game/Blueprints/Environment/BP_LobbyPlayerPlatform.CurrentCharacter` _array_element)))
      (`/Game/ThirdPerson/Blueprints/BP_ThirdPersonCharacter.UpdatePlayerLobbyInfo` _asbp_third_person_character (make `/Game/Blueprints/Characters/S_PlayerLobbyInfo` _requestingplayercontroller (`KismetTextLibrary.Conv_StringToText` (`AdvancedSessionsLibrary.GetPlayerName` _requestingplayercontroller)) (`Controller.PlayerState` _requestingplayercontroller) (`/Game/Blueprints/Controllers/BP_PlayerController_Lobby.bReady` (cast `/Game/Blueprints/Controllers/BP_PlayerController_Lobby` _requestingplayercontroller :!pure true))))
      (`self.CanStartGame`)
      (return)))
  (`/Game/Blueprints/Controllers/BP_PlayerController_Lobby.RetryUpdateLobbyInfo` (cast `/Game/Blueprints/Controllers/BP_PlayerController_Lobby` (`local.RequestingPlayerController`) :!pure true)))

(fn `UpdatePlayersOnPlatforms`
  (locals (IsPlayerAdded :type Boolean))
  (for _array_element (`self.PlayerControllers`)
    (set `local.IsPlayerAdded` false)
    (for _array_element_2 (`self.PlayerPlatforms`)
      (if (== (`/Game/Blueprints/Environment/BP_LobbyPlayerPlatform.PlayerController` _array_element_2) _array_element)
        (set `local.IsPlayerAdded` true)
        (break)))
    (if (not (`local.IsPlayerAdded`))
      (for _array_element_3 (`self.PlayerPlatforms`)
        (`/Engine/EditorBlueprintResources/StandardMacros.IsValid` (`/Game/Blueprints/Environment/BP_LobbyPlayerPlatform.PlayerController` _array_element_3)
          (:`Is Not Valid`
            (`/Game/Blueprints/Environment/BP_LobbyPlayerPlatform.SpawnCharacter` _array_element_3 _array_element)
            (break))))))
  (for _array_element_4 (`self.PlayerPlatforms`)
    (if (not (`KismetArrayLibrary.Array_Contains` (`self.PlayerControllers`) (`/Game/Blueprints/Environment/BP_LobbyPlayerPlatform.PlayerController` _array_element_4)))
      (`/Game/Blueprints/Environment/BP_LobbyPlayerPlatform.RemoveCharacter` _array_element_4))))

(fn `UserConstructionScript`)